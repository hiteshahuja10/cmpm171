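; Boss enemy whose death pauses the game and opens the end-game screen with UI-only input.
; PawnSensing flags the player as seen on the AI controller's blackboard, while a health widget is turned toward the player every tick.
; Attack sphere-traces ahead for the player, plays a montage and applies damage halfway through it.
; HitBoss subtracts health and, at zero, destroys the boss and triggers that end screen.
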(event OnSeePawn(PawnSensing)
  (params (Pawn :type Pawn%20Object%20Reference))
  ;[1 1 1] AI Sense the player
  (Utilities|Casting|CastToBP_FirstPersonCharacter Pawn)
  (AI|Components|Blackboard|SetValueasBool (AI|GetBlackboard (AI|GetAIController self)) (Utilities|Name|MakeLiteralName "HasSeenPlayer?") true))

(event Custom|Attack
  (bind _returnvalue (Transformation|GetActorLocation))
  ;[1 1 1] AI Attack
  (bind (_outhit _returnvalue_2) (Collision|SphereTraceForObjects _returnvalue (+ _returnvalue (* (Math|Vector|GetForwardVector (Transformation|GetActorRotation)) 2.5e+02)) 6e+02 (Utilities|Array|MakeArray "ObjectTypeQuery3") false 0 "None"))
  (if _returnvalue_2
    (Utilities|Casting|CastToBP_FirstPersonCharacter (.HitActor (Collision|BreakHitResult _outhit))
      (:then
        (Development|PrintString "Successfully Attack")
        (bind _returnvalue_3 (Animation|PlayAnimMontage "/Game/MrGoober/animations/MrGoobAttackMontage.MrGoobAttackMontage" 1.0 "None"))
        (Utilities|FlowControl|Delay (* _returnvalue_3 0.5))
        (Game|Damage|ApplyDamage (.HitActor (Collision|BreakHitResult _outhit)) 1e+01 0 0))
      (:CastFailed
        (Development|PrintString "attack failed")))))

(event EventTick
  (params (DeltaSeconds :type Float%20%28single-precision%29))
  (Transformation|SetWorldRotation (Variables|Default|GetWidget) (Math|Rotator|FindLookatRotation (Transformation|GetWorldLocation (Variables|Default|GetWidget)) (Transformation|GetActorLocation (Game|GetPlayerCharacter 0))) false false))

(event EventBeginPlay
  (Variables|Default|SetHealth (Variables|Default|GetMaxHealth))
  (bind _asui_boss_health (Utilities|Casting|CastToUI_BossHealth (UserInterface|GetWidget (Variables|Default|GetWidget))))
  (Variables|/Game/UI/UI_EnemyHealthBar/UI_BossHealth.UI_BossHealth_C|SetUnit%202 _asui_boss_health self))

(event EventHitBoss
  (params (Damage%201%20 :type Float%20%28double-precision%29))
  (bind _returnvalue (Game|GetPlayerController 0))
  (bind _output_get (Variables|Default|SetHealth (- (Variables|Default|GetHealth) Damage%201%20)))
  (if (<= _output_get 0.0)
    (Development|PrintString "Enemy Killed")
    (Actor|DestroyActor)
    (Game|SetGamePaused true)
    (bind _returnvalue_2 (UserInterface|CreateWidget "/Game/UI/UI_EndGame.UI_EndGame_C" _returnvalue))
    (UserInterface|Viewport|AddtoViewport _returnvalue_2 0)
    (Input|SetInputModeUIOnly _returnvalue _returnvalue_2 "DoNotLock" false)
    (Variables|/Script/Engine.PlayerController|SetbShowMouseCursor _returnvalue true)
    (else
      (Utilities|FlowControl|Sequence
        (:then_0
          (Development|PrintString (Utilities|String|ToString(Float) _output_get)))))))

(fn ConstructionScript)