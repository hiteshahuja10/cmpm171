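; Cubes_BP is an AI enemy that flags the blackboard when PawnSensing spots the player, and carries a health bar widget that turns toward them.
; AttackPlayer sphere-traces ahead, plays a tiger attack montage and applies damage halfway through it.
; Projectile overlaps on the cube award the player a point and play a hit sound.
; HitEnemy subtracts the player's damage value, destroying the enemy and spawning a Bubbledgoober at zero health.
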(event OnSeePawn(PawnSensing)
  (params (Pawn :type Pawn%20Object%20Reference))
  ;[1 1 1] Chase Player
  (bind _asbp_first_person_character (Utilities|Casting|CastToBP_FirstPersonCharacter Pawn))
  (Variables|Default|SetChar _asbp_first_person_character)
  (AI|Components|Blackboard|SetValueasBool (AI|GetBlackboard (AI|GetAIController self)) (Utilities|Name|MakeLiteralName "HasSeenPlayer") true))

(event OnComponentBeginOverlap(Cube)
  (params (OverlappedComponent :type Primitive%20Component%20Object%20Reference) (OtherActor :type Actor%20Object%20Reference) (OtherComp :type Primitive%20Component%20Object%20Reference) (OtherBodyIndex :type Integer) (bFromSweep :type Boolean) (SweepResult :type Hit%20Result%20Structure%20%28by%20ref%29))
  (bind _char (Variables|Default|GetChar))
  (Utilities|Casting|CastToBP_FirstPersonProjectile OtherActor)
  (Variables|/Game/FirstPerson/Blueprints/BP_FirstPersonCharacter.BP_FirstPersonCharacter_C|SetPoints _char (+ (Variables|/Game/FirstPerson/Blueprints/BP_FirstPersonCharacter.BP_FirstPersonCharacter_C|GetPoints _char) 1))
  (Audio|PlaySoundatLocation "/Game/Sound/hit.hit" (Transformation|GetActorLocation) "0, 0, 0" 1.0 1.0 0.0 0 0 0 0))

(event Custom|Attack%20Player
  (bind _returnvalue (Transformation|GetActorLocation))
  (Variables|Default|SetcanAttack? true)
  (bind _outhit (Collision|SphereTraceForObjects _returnvalue (+ _returnvalue (* (Math|Vector|GetForwardVector (Transformation|GetActorRotation)) 2.5e+02)) 1.2e+02 (Utilities|Array|MakeArray "ObjectTypeQuery3") false 0 "None"))
  ;[1 1 1] Tiger Attack Animation
  (if (Variables|Default|GetcanAttack?)
    (Utilities|Casting|CastToBP_FirstPersonCharacter (.HitActor (Collision|BreakHitResult _outhit)))
    (Development|PrintString "Attacking")
    (Variables|Default|SetcanAttack? false)
    (bind _returnvalue_2 (Animation|PlayAnimMontage "/Game/Tiger_Mob/animations/TigerAttack__Montage.TigerAttack__Montage" 1.0 "None"))
    (Utilities|FlowControl|Delay (* _returnvalue_2 0.5))
    (Game|Damage|ApplyDamage (.HitActor (Collision|BreakHitResult _outhit)) 1e+01 0 0)
    (Variables|Default|SetcanAttack? true)))

(event EventHitEnemy
  (params (Damage :type Float%20%28double-precision%29))
  (bind _returnvalue (Actor|GetActorOfClass "/Game/FirstPerson/Blueprints/BP_FirstPersonCharacter.BP_FirstPersonCharacter_C"))
  (bind _output_get (Variables|Default|SetHealth (- (Variables|Default|GetHealth) (Variables|/Game/FirstPerson/Blueprints/BP_FirstPersonCharacter.BP_FirstPersonCharacter_C|GetdamageNUM _returnvalue))))
  (if (<= _output_get 0.0)
    (Development|PrintString "Enemy Killed")
    (Actor|DestroyActor)
    (Game|SpawnActorfromClass "/Game/Cube_guy/bubbledgoober.bubbledgoober_C" (Transformation|GetActorTransform) "AdjustIfPossibleButAlwaysSpawn" 0 "0.000000,0.000000,0.000000" "0.000000,0.000000,1000.000000" 0)
    (else
      (Utilities|FlowControl|Sequence
        (:then_0
          (Development|PrintString (Utilities|String|ToString(Float) _output_get)))))))

(event EventTick
  (params (DeltaSeconds :type Float%20%28single-precision%29))
  (Transformation|SetWorldRotation (Variables|Default|GetWidget) (Math|Rotator|FindLookatRotation (Transformation|GetWorldLocation (Variables|Default|GetWidget)) (Transformation|GetActorLocation (Game|GetPlayerCharacter 0))) false false))

(event EventBeginPlay
  (Variables|Default|SetHealth (Variables|Default|GetMaxHealth))
  (bind _asui_health_bar (Utilities|Casting|CastToUI_HealthBar (UserInterface|GetWidget (Variables|Default|GetWidget))))
  (Variables|/Game/UI/UI_EnemyHealthBar/UI_HealthBar.UI_HealthBar_C|SetUnit _asui_health_bar self))

(fn ConstructionScript)